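; Test trigger actor that plays a sound through the player's commander audio the first time the player overlaps it.
; A first-enter flag is set on BeginPlay and cleared once playback starts, so the trigger fires only once.
; On overlap by player pawn 0, it assigns its sound to the PPCharacterPlayer's CommanderAudioComponent and plays it.
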(event EventBeginPlay
  (Variables|Default|SetFirstEnter true))

(event Collision|EventActorBeginOverlap
  (params (OtherActor :type Actor%20Object%20Reference))
  (bind _returnvalue (Game|Player|GetPlayerPawn 0))
  (if (Variables|Default|GetFirstEnter)
    (bind _asppcharacter_player (Utilities|Casting|CastToPPCharacterPlayer _returnvalue))
    (if (== _returnvalue OtherActor)
      (Audio|Components|Audio|SetSound (Variables|/Script/ProjectP.PPCharacterPlayer|GetCommanderAudioComponent _asppcharacter_player) (Variables|Default|GetSound))
      (Audio|Components|Audio|Play (Variables|/Script/ProjectP.PPCharacterPlayer|GetCommanderAudioComponent _asppcharacter_player) (Variables|Default|GetStartTime))
      (Variables|Default|SetFirstEnter false))))

(event EventTick
  (params (DeltaSeconds :type Float%20%28single-precision%29)))

(fn ConstructionScript)