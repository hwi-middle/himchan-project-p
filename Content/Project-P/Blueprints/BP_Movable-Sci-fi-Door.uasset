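; Movable sci-fi double door that slides open when the player character overlaps the actor and closes when the overlap ends.
; BeginPlay caches both panels' relative positions, then the DoorMove timeline adds a vector curve to them, with Y negated for the right panel.
; An IsMoving flag blocks new play or reverse requests mid-motion, retrying each second through a Delay loop until the door stops.
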(event Collision|EventActorBeginOverlap
  (params (OtherActor :type Actor%20Object%20Reference))
  (if (== OtherActor (Game|GetPlayerCharacter 0))
    (if (Variables|Default|GetIsMoving) :!label _label
      (Utilities|FlowControl|Delay 1.0)
      (goto _label)
      (else
        (bind _door_open_curve (Timeline|DoorMove Play)
          (:Update
            (Utilities|FlowControl|Sequence
              (:then_0
                (Variables|Default|SetIsMoving true))
              (:then_1
                (Transformation|SetRelativeLocation (Variables|Default|Getdoor_left) (+ _door_open_curve (Variables|Default|GetLeft%20Origin%20Position)) false false))
              (:then_2
                (Transformation|SetRelativeLocation (Variables|Default|Getdoor_right) (+ (* _door_open_curve "1.000000,-1.000000,1.000000") (Variables|Default|GetRight%20Origin%20Position)) false false))))
          (:Finished
            (Variables|Default|SetIsMoving false)))))))

(event Collision|EventActorEndOverlap
  (params (OtherActor :type Actor%20Object%20Reference))
  (if (== OtherActor (Game|GetPlayerCharacter 0))
    (if (Variables|Default|GetIsMoving) :!label _label
      (Utilities|FlowControl|Delay 1.0)
      (goto _label)
      (else
        (bind _door_open_curve (Timeline|DoorMove Reverse)
          (:Update
            (Utilities|FlowControl|Sequence
              (:then_0
                (Variables|Default|SetIsMoving true))
              (:then_1
                (Transformation|SetRelativeLocation (Variables|Default|Getdoor_left) (+ _door_open_curve (Variables|Default|GetLeft%20Origin%20Position)) false false))
              (:then_2
                (Transformation|SetRelativeLocation (Variables|Default|Getdoor_right) (+ (* _door_open_curve "1.000000,-1.000000,1.000000") (Variables|Default|GetRight%20Origin%20Position)) false false))))
          (:Finished
            (Variables|Default|SetIsMoving false)))))))

(event EventBeginPlay
  (Variables|Default|SetLeft%20Origin%20Position (Variables|/Script/Engine.SceneComponent|GetRelativeLocation (Variables|Default|Getdoor_left)))
  (Variables|Default|SetRight%20Origin%20Position (Variables|/Script/Engine.SceneComponent|GetRelativeLocation (Variables|Default|Getdoor_right))))

(fn ConstructionScript)