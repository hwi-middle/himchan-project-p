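; BP_Trigger_Capsule is a glass capsule actor that shatters when its PPDestructible component fires DestructDelegate.
; BeginPlay hides the second glass mesh and the geometry-collection glass, leaving the latter query-only.
; On destruct it destroys the first glass component, reveals both hidden ones and triggers Chaos destruction through ChaosDestruction.
; After a delay it hides the fractured glass and only then plays the 2D glass-break sound.
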(event DestructDelegate(PPDestructible)
  (Components|DestroyComponent (Variables|Default|GetSM_Capsule_Glass01))
  (Rendering|SetVisibility (Variables|Default|GetSM_Capsule_Glass02) true false)
  (Rendering|SetVisibility (Variables|Default|GetSM_Capsule_Glass01_GCOnly_GC) true false)
  (Default|CETrigger (Variables|Default|GetChaos%20Destruction))
  (Utilities|FlowControl|Delay 5.0)
  (Rendering|SetVisibility (Variables|Default|GetSM_Capsule_Glass01_GCOnly_GC) false false)
  (Audio|PlaySound2D "/Game/Project-P/Sound/SFX/MS_GalssDestroy_Cue.MS_GalssDestroy_Cue" 1.0 1.0 0.0 0 0))

(event EventBeginPlay
  (bind _sm_capsule_glass01_gconly_gc (Variables|Default|GetSM_Capsule_Glass01_GCOnly_GC))
  (Rendering|SetVisibility (Variables|Default|GetSM_Capsule_Glass02) false false)
  (Rendering|SetVisibility _sm_capsule_glass01_gconly_gc false false)
  (Collision|SetCollisionEnabled _sm_capsule_glass01_gconly_gc "QueryOnly"))

(event Collision|EventActorBeginOverlap
  (params (OtherActor :type Actor%20Object%20Reference)))

(event EventTick
  (params (DeltaSeconds :type Float%20%28single-precision%29)))

(fn ConstructionScript)